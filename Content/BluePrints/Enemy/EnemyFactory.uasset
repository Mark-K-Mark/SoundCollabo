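; Enemy factory that spawns random enemies inside a spawn area while the GameManager's scene matches the game state.
; Its Action event draws the area's debug box and, unless the factory sits at the world origin, spawns one of three enemy classes on a frame-count interval, up to a cap.
; Before spawning, it destroys and unlists enemies in Point or Damage state, counting only Point as a defeat.
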(event EventAction
  (bind _spawnarea (Variables|Default|GetSpawnArea))
  (bind _spawnarea_2 (Variables|Default|GetSpawnArea))
  (bind _enemy (Variables|Default|GetEnemy))
  (bind _returnvalue (Transformation|GetActorTransform _spawnarea_2))
  (bind (_origin _boxextent) (Collision|GetActorBounds _spawnarea false))
  ;[1 1 1] 敵生成範囲の移動
  (Variables|Default|SetCountFlame (+ (Variables|Default|GetCountFlame) 1))
  (Rendering|Debug|DrawDebugBox (.location _returnvalue) (.BoxExtent (Collision|GetActorBounds _spawnarea_2 false)) "(R=1.000000,G=0.127075,B=0.111111,A=1.000000)" (.rotation _returnvalue) 0.0 0.0) ; 敵生成エリアデバッグ表示
  (if (Math|Vector|Equal(Vector) (Transformation|GetActorLocation) "0, 0, 0" 0.0001) ; EndPosに到着しているかどうか
    (Variables|Default|SetUpdate false)
    (else
      ;[1 1 1] 敵の生成
      (CallFunction|IsAlivedEnemy _enemy) ; エネミーの生存確認
      (if (Utilities|Enum|Equal(Enum) (Variables|/Game/BluePrints/GameManager/GameManager.GameManager_C|GetnowScene (Variables|Default|GetgameMgr)) "NewEnumerator1") ; 現在シーンがGame時に生成
        (if (< (Utilities|Array|Length _enemy) (Variables|Default|GetMaxSpawn)) ; 敵の数が範囲内なら
          (if (== (Variables|Default|GetSpawnInterval) (Variables|Default|GetCountFlame)) ; インターバルのフレーム数なら
            (bind _returnvalue_2 (Game|SpawnActorfromClass (Utilities|Array|Get(acopy) (Variables|Default|GetSpawnEnemy) (Math|Random|RandomIntegerinRange 0 2)) (Math|Transform|MakeTransform (Math|Random|RandomPointinBoundingBox _origin _boxextent)) "Undefined" 0 0))
            (Utilities|Array|Add (Variables|Default|GetEnemy) _returnvalue_2)
            (Variables|Default|SetCountFlame 0)
            (Variables|Default|SetSpawnCounter (+ (Variables|Default|GetSpawnCounter) 1)))
          (else
            (Variables|Default|SetCountFlame 0)))))))

(event EventTick
  (params (DeltaSeconds :type Float%20%28single-precision%29))
  (|CallParentFunction DeltaSeconds))

(fn ConstructionScript
  (bind _spawnenemy (Variables|Default|GetSpawnEnemy))
  (|CallParentFunction)
  ;[1 1 1] GameManager取得
  (bind _outactors (Actor|GetAllActorsOfClass "/Game/BluePrints/GameManager/GameManager.GameManager_C"))
  (Variables|Default|SetgameMgr (Utilities|Array|Get(acopy) _outactors))
  (Utilities|FlowControl|Sequence
    (:then_0
      (Utilities|Array|Add _spawnenemy "/Game/BluePrints/Enemy/Enemy_1.Enemy_1_C"))
    (:then_1
      (Utilities|Array|Add _spawnenemy "/Game/BluePrints/Enemy/Enemy_2.Enemy_2_C"))
    (:then_2
      (Utilities|Array|Add _spawnenemy "/Game/BluePrints/Enemy/Enemy_3.Enemy_3_C"))))

(fn IsAlivedEnemy
  (params (Enemy :type Array%20of%20Actor%20Object%20References))
  (for (_array_element _array_index) Enemy
    (bind _asenemy (Utilities|Casting|CastToEnemy _array_element))
    (if (Utilities|IsValid _asenemy) ; インスタンスが削除されていなければ
      (switch Utilities|FlowControl|Switch|SwitchonEnemyDieState (Variables|/Game/BluePrints/Enemy/Enemy.Enemy_C|GetEnemyState _asenemy)
        (:NewEnumerator0
          (Variables|Default|SetDefeatCount (+ (Variables|Default|GetDefeatCount) 1)))
        (:NewEnumerator1
          _))
      (Utilities|Array|RemoveIndex Enemy _array_index)
      (Actor|DestroyActor _asenemy))))