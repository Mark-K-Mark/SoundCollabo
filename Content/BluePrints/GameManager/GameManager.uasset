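; GameManager runs the game's Title, Game and Result flow as a state switch on Tick, with its own Fire input enabled only outside gameplay.
; Firing on the title activates all GameObjects and swaps title UI for score UI.
; During play it copies EnemyFactory's defeat count until time expires, then spawns Result before the camera.
; Result converts score to percent of spawned enemies, ranks it S to C, and reloads the level on Fire.
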(event EventTick
  (params (DeltaSeconds :type Float%20%28single-precision%29))
  ;[1 1 1] Tick
  (switch Utilities|FlowControl|Switch|SwitchonEScene (Variables|Default|GetnowScene)
    (:NewEnumerator0
      (|TitleTick))
    (:NewEnumerator1
      (Variables|Default|SetTotalTime (+ DeltaSeconds (Variables|Default|GetTotalTime)))
      (|GameTick))
    (:NewEnumerator2
      (|ResultTick))))

(event EventBeginPlay
  ;[1 1 1] タイトル用にこのクラスでキー入力出来る様にする
  (Input|EnableInput (Game|GetPlayerController 0))
  (Audio|Components|Audio|Play (Variables|Default|GetTitleBGM) 0.0))

(event Input|ActionEvents|InputActionFire
  (params (Key :type Key%20Structure))
  (:Pressed
    (Variables|Default|SetisFire true))
  (:Released
    (Variables|Default|SetisFire false)))

(fn ConstructionScript
  (Variables|Default|SetrankBorderS 90)
  (Variables|Default|SetrankBorderA 60)
  (Variables|Default|SetrankBorderB 30)
  (Variables|Default|SetresultScene "NewEnumerator0"))

(fn ScoretoPercent
  (params (score :type Integer))
  (bind _outactors (Actor|GetAllActorsOfClass "/Game/BluePrints/Enemy/EnemyFactory.EnemyFactory_C"))
  (return (Math|Float|Truncate (* (/ (Math|Conversions|ToFloat(Integer) (Variables|Default|Getscore)) (Math|Conversions|ToFloat(Integer) (Variables|/Game/BluePrints/Enemy/EnemyFactory.EnemyFactory_C|GetSpawnCounter (Utilities|Array|Get(acopy) _outactors)))) 1e+02))))