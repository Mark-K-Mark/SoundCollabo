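; Actor component that moves and rotates its owner along an assigned spline at a set speed.
; Tick advances a travel distance and ForceMove applies the spline's transform at that point to the owner.
; At an end, Return and Loop select stopping, wrapping, a single round trip or endless ping-pong, with stopping done by disabling tick.
; Helpers set the spline, adjust distance and pause movement; GetNowLenPercentage returns length modulo distance, not a percentage.
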(event EventBeginPlay)

(event EventTick
  (params (DeltaSeconds :type Float%20%28single-precision%29))
  (Variables|Default|SetMoveDistance (+ (Variables|Default|GetMoveDistance) (* DeltaSeconds (Variables|Default|GetSpeed))))
  (CallFunction|ForceMove)
  (if (CallFunction|IsArrived)
    (if (Variables|Default|GetReturn) ; 反転するかどうか
      (if (and (not (Variables|Default|GetLoop)) (<= (Variables|Default|GetMoveDistance) 0.0)) ; 始点かどうか
        (Components|Tick|SetComponentTickEnabled false) ; 反転移動終了
        (else
          ;[1 1 1] 進行方向を逆にする
          (Variables|Default|SetSpeed (* (Variables|Default|GetSpeed) -1.0))
          (Variables|Default|SetReverse (not (Variables|Default|GetReverse)))))
      (elif (Variables|Default|GetLoop) ; ループするかどうか
        (Variables|Default|SetMoveDistance (- (Variables|Default|GetMoveDistance) (CallFunction|GetSplineLength)))
        (else
          (Components|Tick|SetComponentTickEnabled false) ; 移動終了
        )))))

(fn SetSpline
  (params (Spline :type Spline%20Actor%20Object%20Reference%20%28by%20ref%29))
  (Variables|Default|SetSpline Spline)
  (Variables|Default|SetMoveDistance 0.0))

(fn IsArrived
  (if (Variables|Default|GetReverse)
    (LocalVariables|Setarrived (<= (Variables|Default|GetMoveDistance) 0.0))
    (else
      (LocalVariables|Setarrived (Default|IsArrived (Variables|Default|GetSpline) (Variables|Default|GetMoveDistance)))))
  (return (LocalVariables|Getarrived)))

(fn SetMoveDistance
  (params (distance :type Float%20%28single-precision%29))
  (Variables|Default|SetMoveDistance distance))

(fn AddMoveDistance
  (params (Distance :type Float%20%28single-precision%29))
  (CallFunction|SetMoveDistance (+ Distance (Variables|Default|GetMoveDistance))))

(fn ForceMove
  (bind _return (Variables|Default|GetReturn))
  (bind _loop (Variables|Default|GetLoop))
  (bind _spline (Variables|Default|GetSpline))
  (bind _movedistance (Variables|Default|GetMoveDistance))
  (bind _returnvalue (not _return))
  (bind _returnvalue_2 (and _loop _returnvalue))
  (bind (_location _rotation) (Default|GetCurrentLocationandRotation _spline _movedistance _returnvalue_2))
  (Transformation|SetActorLocationAndRotation (Components|GetOwner) _location _rotation))

(fn Pause
  (params (IsPause :type Boolean))
  (Components|Tick|SetComponentTickEnabled (not IsPause)))

(fn GetSplineLength
  (return (Default|GetSplineLength (Variables|Default|GetSpline))))

(fn GetNowLenPercentage
  (return (Math|Float|%(Float) (Default|GetSplineLength (Variables|Default|GetSpline)) (Variables|Default|GetMoveDistance))))