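; UFO enemy that flies with slight random drift while spinning, built on a parent enemy class.
; Construction offsets, turns and scales it, picks its direction and sets its score; BeginPlay adds spawn effect and sound.
; Tick accumulates per-frame movement in MoveTrans, unscaled by delta time, and composes yaw spin separately so the path stays straight.
; Gun overlap changes EnemyState and shakes the camera; hits go to EnemyEventHit.
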(event EventBeginPlay
  (|CallParentFunction)
  (Game|SpawnActorfromClass "/Game/BluePrints/Enemy/BP_EnemySpownEffect_UFO.BP_EnemySpownEffect_UFO_C" (Math|Transform|MakeTransform (Transformation|GetWorldLocation (Variables|Default|GetDefaultSceneRoot)) "0, 0, 0" "1.000000,1,1") "Undefined" 0 0)
  (Audio|Components|Audio|Play (Variables|Default|GetUFOAudio) 0.0 :!pinned true) ; UFOのSE再生
)

(event EventTick
  (params (DeltaSeconds :type Float%20%28single-precision%29))
  (|CallParentFunction DeltaSeconds)
  (bind _output_get (Variables|Default|SetmoveTrans (Math|Transform|ComposeTransforms (Math|Transform|MakeTransform (* (Variables|Default|GetmoveDirection) (Variables|Default|Getspeed))) (Variables|Default|GetmoveTrans)))) ; 移動Transform更新
  (if (<= (+ (Variables|Default|GetnowRot) (Variables|Default|GetaddRot)) 3.6e+02) ; 一応360以いかないようにする
    (Variables|Default|SetnowRot (+ (Variables|Default|GetnowRot) (Variables|Default|GetaddRot)))
    (else
      (Variables|Default|SetnowRot (- (+ (Variables|Default|GetnowRot) (Variables|Default|GetaddRot)) 3.6e+02))))
  (Transformation|SetActorTransform (Math|Transform|ComposeTransforms (Math|Transform|MakeTransform "0, 0, 0" (Math|Rotator|MakeRotator 0.0 0.0 (Variables|Default|GetnowRot))) _output_get)))

(event Collision|EventHit
  (params (MyComp :type Primitive%20Component%20Object%20Reference) (Other :type Actor%20Object%20Reference) (OtherComp :type Primitive%20Component%20Object%20Reference) (bSelfMoved :type Boolean) (HitLocation :type Vector :default "0, 0, 0") (HitNormal :type Vector :default "0, 0, 0") (NormalImpulse :type Vector :default "0, 0, 0") (Hit :type Hit%20Result%20Structure%20%28by%20ref%29))
  (CallFunction|EnemyEventHit Other HitLocation))

(event Collision|EventActorBeginOverlap
  (params (OtherActor :type Actor%20Object%20Reference))
  (if (== (Utilities|GetClass OtherActor) "/Game/BluePrints/Player/Gun.Gun_C")
    (Variables|Default|SetEnemyState "NewEnumerator1")
    (Class|PlayerController|ClientPlayCameraShake (Game|GetPlayerController 0) "/Game/BluePrints/Generic/CameraShake/PlayerCameraShake.PlayerCameraShake_C" 1.0 "CameraLocal" "0, 0, 0")))

(fn ConstructionScript
  (|CallParentFunction)
  (Transformation|SetActorTransform (Math|Transform|ComposeTransforms (Math|Transform|MakeTransform "3000.000000, 0, 0" "0,180.000000, 0" "5.500000,5.500000,5.500000") (Transformation|GetActorTransform)))
  (Variables|Default|SetmoveDirection (Math|Vector|MakeVector 1.0 (Math|Random|RandomFloatinRange -0.2 0.2) (Math|Random|RandomFloatinRange -0.2 0.2)))
  (Variables|Default|SetmoveTrans (Transformation|GetActorTransform))
  (Variables|Default|SetaddScore 1000))