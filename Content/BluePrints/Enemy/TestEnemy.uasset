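; TestEnemy is a test enemy actor that homes in on the player's Gun actor while spinning.
; Construction script caches the first Gun found and seeds a movement transform from the actor's own transform.
; Each Tick advances that transform a fixed step along its forward axis, re-aims it with RInterpTo, then composes a growing local yaw spin onto it.
; An unconnected chain holds a simpler rotate-and-offset version.
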(event EventBeginPlay
  (|CallParentFunction) ; This node is disabled and will not be called.\nDrag off pins to build functionality.
)

(event Collision|EventActorBeginOverlap
  (params (OtherActor :type Actor%20Object%20Reference))
  (|CallParentFunction OtherActor))

(event EventTick
  (params (DeltaSeconds :type Float%20%28single-precision%29))
  (|CallParentFunction DeltaSeconds)
  (bind _output_get (Variables|Default|SetrotationZPow (+ (Variables|Default|GetrotationZPow) 1e+01)))
  (bind _output_get_2 (Variables|Default|SetMoveTrans (Math|Transform|MakeTransform (Math|Transform|TransformLocation (Variables|Default|GetMoveTrans) "10.000000, 0, 0") (Math|Interpolation|RInterpTo (Transformation|GetActorRotation) (Math|Rotator|FindLookatRotation (Transformation|GetActorLocation) (Transformation|GetActorLocation (Variables|Default|GetGunActor))) (Utilities|Time|GetWorldDeltaSeconds) 1e+02))))
  (Transformation|SetActorTransform (Math|Transform|ComposeTransforms (Math|Transform|MakeTransform "0,0.000000, 0" (Math|Rotator|MakeRotator 0.0 0.0 _output_get)) _output_get_2)))

(fn ConstructionScript
  (|CallParentFunction)
  (bind _outactors (Actor|GetAllActorsOfClass "/Game/BluePrints/Player/Gun.Gun_C")) ; Gun(Player)を検索して\nGunActorへセット
  (Variables|Default|SetGunActor (Utilities|Array|Get(acopy) _outactors))
  (Variables|Default|SetMoveTrans (Transformation|GetActorTransform)) ; 移動用の行列セット
)