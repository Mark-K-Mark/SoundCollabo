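; First-person player gun Blueprint with a charge shot, supporting VR motion controllers and keyboard/mouse look.
; Holding Fire accumulates charge time and scales a preview bullet at the right gun, reusing the first FirstPersonProjectile_P found by the construction script.
; Releasing Fire spawns a charge-scaled projectile from the gun when the right controller tracks, otherwise from the camera.
; VR setup disables controller yaw and can hide the unused mesh.
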(event EventBeginPlay
  ;[1 1 1] HMDを使用する場合、VRモードで使用しないメッシュを消す
  (if (Class|HeadMountedDisplayFunctionLibrary|IsHeadMountedDisplayEnabled)
    (Variables|Default|SetbUseControllerRotationYaw false)
    (if (Variables|Default|GetUsingMotionControllers)
      (Development|SetHiddeninGame (Variables|MyCharacter|GetMesh2P) true true))))

(event EventTick
  (params (DeltaSeconds :type Float%20%28single-precision%29))
  (Variables|Default|SetUsingMotionControllers (Class|MotionControllerComponent|IsTracked (Variables|Default|GetR_MotionController)))
  (if (Variables|Default|GetChargeFlag)
    (Variables|Default|SetChargeTime (+ DeltaSeconds (Variables|Default|GetChargeTime)))
    (bind _output_get (Variables|Default|SetShotCenter (Math|Transform|MakeTransform (+ (Transformation|GetWorldLocation (Variables|Default|GetRightGun)) (Math|Vector|RotateVector (Variables|Default|GetGunOffset) (Transformation|GetWorldRotation (Variables|Default|GetR_MotionController)))) (Transformation|GetWorldRotation (Variables|Default|GetBaseNode)) (Math|Vector|MakeVector (Math|Float|Clamp(Float) (+ (Variables|Default|GetChargeTime) 1.0) 0.0 (Variables|Default|GetMAX_CHARGE)) (Math|Float|Clamp(Float) (+ (Variables|Default|GetChargeTime) 1.0) 0.0 (Variables|Default|GetMAX_CHARGE)) (Math|Float|Clamp(Float) (+ (Variables|Default|GetChargeTime) 1.0) 0.0 (Variables|Default|GetMAX_CHARGE))))))
    (Transformation|SetActorTransform (Variables|Default|GetBullet) _output_get)
    (Development|SetHiddeninGame (Variables|Default|GetRay) (Variables|Default|GetNotGame) false)
    (else
      (Variables|Default|SetChargeTime 0.0))))

(event Input|ActionEvents|InputActionResetVR
  (params (Key :type Key%20Structure))
  ;[1 1 1] VRの座標と視点をリセットする
  (:Pressed
    (Class|HeadMountedDisplayFunctionLibrary|ResetOrientationandPosition 0.0 "OrientationAndPosition")))

(event Input|ActionEvents|InputActionFire
  (params (Key :type Key%20Structure))
  (bind _firstpersoncamera (Variables|MyCharacter|GetFirstPersonCamera))
  (bind _bullet (Variables|Default|GetBullet))
  (bind _chargetime (Variables|Default|GetChargeTime))
  (bind _max_charge (Variables|Default|GetMAX_CHARGE))
  (bind _charge (Variables|Default|GetCharge))
  (bind _returnvalue (Transformation|GetWorldTransform _firstpersoncamera))
  (bind _returnvalue_2 (+ _chargetime 1.0))
  (bind _returnvalue_3 (Math|Float|Clamp(Float) _returnvalue_2 0.0 _max_charge))
  (bind (_location _rotation) (Math|Transform|BreakTransform _returnvalue))
  (bind _returnvalue_4 (Math|Vector|MakeVector _returnvalue_3 _returnvalue_3 _returnvalue_3))
  ;[1 1 1] 弾の生成
  (:Pressed
    (if (Math|Boolean|Equal(Boolean) (Variables|Default|GetChargeFlag) true)
      _
      (else
        (Audio|Components|Audio|Play _charge 0.0)
        (Rendering|SetActorHiddenInGame _bullet false)))
    (Variables|Default|SetChargeFlag true))
  (:Released
    (Variables|Default|SetChargeFlag false)
    (Animation|Montage|MontagePlay (Components|SkeletalMesh|GetAnimInstance (Variables|MyCharacter|GetMesh2P)) "/Game/FirstPerson/Animations/FirstPersonFire_Montage.FirstPersonFire_Montage" 1.0 "MontageLength" 0.0 true)
    (Audio|Components|Audio|Stop _charge)
    (Rendering|SetActorHiddenInGame _bullet true)
    (Game|SpawnActorfromClass "/Game/BluePrints/Player/FirstPersonProjectile.FirstPersonProjectile_C" (select (Variables|Default|GetUsingMotionControllers) (Math|Transform|MakeTransform (+ (Transformation|GetWorldLocation (Variables|Default|GetRightGun)) (Math|Vector|RotateVector (Variables|Default|GetGunOffset) (Transformation|GetWorldRotation (Variables|Default|GetR_MotionController)))) (Transformation|GetWorldRotation (Variables|Default|GetBaseNode)) _returnvalue_4) (Math|Transform|MakeTransform _location _rotation _returnvalue_4)) "AdjustIfPossibleButDontSpawnIfColliding" 0 0) ; 弾の生成
    (Audio|Components|Audio|Play (Variables|Default|GetFire) 0.0)))

(event Input|AxisEvents|InputAxisTurn
  (params (AxisValue :type Float%20%28single-precision%29))
  ;[1 1 1] マウス入力
  (Pawn|Input|AddControllerYawInput AxisValue))

(event Input|AxisEvents|InputAxisLookUp
  (params (AxisValue :type Float%20%28single-precision%29))
  ;[1 1 1] マウス入力
  (Pawn|Input|AddControllerPitchInput AxisValue))

(event Input|AxisEvents|InputAxisTurnRate
  (params (AxisValue :type Float%20%28single-precision%29))
  ;[1 1 1] キーボード入力
  (Pawn|Input|AddControllerYawInput (* AxisValue (Variables|Default|GetBaseTurnRate) (Utilities|Time|GetWorldDeltaSeconds))))

(fn ConstructionScript
  (Transformation|AttachComponentToComponent (Variables|Default|GetFP_Gun) (Variables|MyCharacter|GetMesh2P) "GripPoint" "SnapToTarget" "SnapToTarget" "SnapToTarget" true)
  (Variables|Default|SetMAX_CHARGE 2.0)
  (Variables|Default|SetMAX_ELERADIUS 15.0)
  (bind _outactors (Actor|GetAllActorsOfClass "/Game/BluePrints/Player/FirstPersonProjectile_P.FirstPersonProjectile_P_C"))
  (Variables|Default|SetBullet (Utilities|Array|Get(acopy) _outactors)))