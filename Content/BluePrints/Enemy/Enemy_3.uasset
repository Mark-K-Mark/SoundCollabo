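; Enemy_3 is an enemy that flies in a straight line roughly toward the player's Gun actor.
; The construction script interpolates its rotation toward the first Gun found, then adds random pitch and yaw offsets.
; After calling the parent Tick, it moves a fixed local-forward step each frame, independent of delta time.
; Projectile hits set EnemyState and spawn an explosion; Gun contact sets another state, with camera shake on overlap only.
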(event EventTick
  (params (DeltaSeconds :type Float%20%28single-precision%29))
  (|CallParentFunction DeltaSeconds)
  (Transformation|SetActorTransform (Math|Transform|ComposeTransforms (Math|Transform|MakeTransform "3.000000, 0, 0") (Transformation|GetActorTransform))))

(event Collision|EventHit
  (params (MyComp :type Primitive%20Component%20Object%20Reference) (Other :type Actor%20Object%20Reference) (OtherComp :type Primitive%20Component%20Object%20Reference) (bSelfMoved :type Boolean) (HitLocation :type Vector :default "0, 0, 0") (HitNormal :type Vector :default "0, 0, 0") (NormalImpulse :type Vector :default "0, 0, 0") (Hit :type Hit%20Result%20Structure%20%28by%20ref%29))
  (bind _returnvalue (Utilities|GetClass Other))
  (if (== _returnvalue "/Game/BluePrints/Player/FirstPersonProjectile.FirstPersonProjectile_C")
    (Variables|Default|SetEnemyState "NewEnumerator0")
    (Effects|SpawnEmitteratLocation "/Game/Architecture/Particle/Explosion/P_EnemyExplosion.P_EnemyExplosion" HitLocation)
    (elif (== _returnvalue "/Game/BluePrints/Player/Gun.Gun_C")
      (Variables|Default|SetEnemyState "NewEnumerator1"))))

(event Collision|EventActorBeginOverlap
  (params (OtherActor :type Actor%20Object%20Reference))
  (if (== (Utilities|GetClass OtherActor) "/Game/BluePrints/Player/Gun.Gun_C")
    (Variables|Default|SetEnemyState "NewEnumerator1")
    (Class|PlayerController|ClientPlayCameraShake (Game|GetPlayerController 0) "/Game/BluePrints/Generic/CameraShake/PlayerCameraShake.PlayerCameraShake_C" 1.0 "CameraLocal" "0, 0, 0")))

(fn ConstructionScript
  (bind _returnvalue (Transformation|GetActorRotation))
  (bind (_roll _pitch _yaw) (Math|Rotator|BreakRotator _returnvalue))
  (|CallParentFunction)
  (bind _outactors (Actor|GetAllActorsOfClass "/Game/BluePrints/Player/Gun.Gun_C")) ; Gun(Player)を検索
  (Transformation|SetActorRotation (Math|Interpolation|RInterpTo (Transformation|GetActorRotation) (Math|Rotator|FindLookatRotation (Transformation|GetActorLocation) (Transformation|GetActorLocation (Utilities|Array|Get(acopy) _outactors))) (Utilities|Time|GetWorldDeltaSeconds) 1e+02) :!pinned true) ; 一旦とりあえず自機方向へ向かせる
  (Transformation|SetActorRotation (Math|Rotator|MakeRotator _roll (+ (Math|Random|RandomFloatinRange -3e+01 3e+01) _pitch) (+ _yaw (Math|Random|RandomFloatinRange -3e+01 3e+01))) :!pinned true) ; 新しく方向をセット
)