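; Spaceship actor that moves steadily forward and trails twin jet effects.
; Each Tick it composes a small local X translation onto its transform without sweep, so speed depends on frame rate.
; It also spawns new left and right jet emitters every frame at fixed world-axis offsets, with auto-destroy off.
; The construction script disables the static mesh's unwanted collision.
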(event EventBeginPlay)

(event Collision|EventActorBeginOverlap
  (params (OtherActor :type Actor%20Object%20Reference)))

(event EventTick
  (params (DeltaSeconds :type Float%20%28single-precision%29))
  (bind _returnvalue (Transformation|GetActorLocation))
  ;[1 1 1] 移動
  (Transformation|SetActorTransform (Math|Transform|ComposeTransforms (Math|Transform|MakeTransform "1.000000, 0, 0") (Transformation|GetActorTransform)))
  ;[1 1 1] ジェット生成
  (Effects|SpawnEmitteratLocation "/Game/Architecture/Mesh/SpaceShip/jet2.jet2" (+ _returnvalue "-280.000000,55.000000,80.000000") "90.000000, 0, 0" "1.000000,1.000000,1.000000" false)
  (Effects|SpawnEmitteratLocation "/Game/Architecture/Mesh/SpaceShip/jet2.jet2" (+ _returnvalue "-280.000000,-55.000000,80.000000") "90.000000, 0, 0" "1.000000,1.000000,1.000000" false))

(fn ConstructionScript
  (Collision|SetCollisionEnabled (Variables|Default|GetStaticMesh) "NoCollision" :!pinned true) ; なぜかコリジョンがついているので削除
)