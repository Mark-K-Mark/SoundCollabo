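; GameManager_Test is a test game manager that switches the game between Title, Game and Result scenes, dispatched each Tick.
; On Title, Fire flags all GameObjects as updating in Game, enables the first Gun's spline tick, removes the TitleLogo and releases input.
; Game's end check is a placeholder fixed to false, so the switch to Result never fires.
; Result would reload the current level on Fire.
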(event EventTick
  (params (DeltaSeconds :type Float%20%28single-precision%29))
  ;[1 1 1] Tick
  (switch Utilities|FlowControl|Switch|SwitchonEScene (Variables|Default|GetnowScene)
    (:NewEnumerator0
      (|TitleTick))
    (:NewEnumerator1
      (|GameTick))
    (:NewEnumerator2
      (|ResultTick))))

(event EventBeginPlay
  ;[1 1 1] タイトル用にこのクラスでキー入力出来る様にする
  (Input|EnableInput (Game|GetPlayerController 0)))

(event Input|ActionEvents|InputActionFire
  (params (Key :type Key%20Structure))
  (:Pressed
    (Variables|Default|SetisFire true))
  (:Released
    (Variables|Default|SetisFire false)))

(fn ConstructionScript)