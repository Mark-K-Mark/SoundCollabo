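; Temporary enemy Blueprint that tracks whether it is alive, was shot by the player or struck the gun.
; A FirstPersonProjectile hit sets Point and spawns an explosion at the impact, while a Gun hit or overlap sets Damage, with overlap also shaking the player camera.
; The construction script starts it as Alive, and IsAlived reports false for both Point and Damage without destroying the actor here.
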(event EventBeginPlay)

(event Collision|EventHit
  (params (MyComp :type Primitive%20Component%20Object%20Reference) (Other :type Actor%20Object%20Reference) (OtherComp :type Primitive%20Component%20Object%20Reference) (bSelfMoved :type Boolean) (HitLocation :type Vector :default "0, 0, 0") (HitNormal :type Vector :default "0, 0, 0") (NormalImpulse :type Vector :default "0, 0, 0") (Hit :type Hit%20Result%20Structure%20%28by%20ref%29))
  (bind _returnvalue (Utilities|GetClass Other))
  (if (== _returnvalue "/Game/BluePrints/Player/FirstPersonProjectile.FirstPersonProjectile_C")
    (Variables|Default|SetEnemyState "NewEnumerator0")
    (Effects|SpawnEmitteratLocation "/Game/Architecture/Particle/Explosion/P_EnemyExplosion.P_EnemyExplosion" HitLocation)
    (elif (== _returnvalue "/Game/BluePrints/Player/Gun.Gun_C")
      (Variables|Default|SetEnemyState "NewEnumerator1"))))

(event Collision|EventActorBeginOverlap
  (params (OtherActor :type Actor%20Object%20Reference))
  (if (== (Utilities|GetClass OtherActor) "/Game/BluePrints/Player/Gun.Gun_C")
    (Variables|Default|SetEnemyState "NewEnumerator1")
    (Class|PlayerController|ClientPlayCameraShake (Game|GetPlayerController 0) "/Game/BluePrints/Generic/CameraShake/PlayerCameraShake.PlayerCameraShake_C" 1.0 "CameraLocal" "0, 0, 0")))

(fn ConstructionScript
  (Variables|Default|SetEnemyState "NewEnumerator3"))

(fn IsAlived
  (switch Utilities|FlowControl|Switch|SwitchonEnemyDieState (Variables|Default|GetEnemyState)
    (:NewEnumerator0
      _)
    (:NewEnumerator1
      _)
    (:NewEnumerator3
      (return true)))
  (return false))