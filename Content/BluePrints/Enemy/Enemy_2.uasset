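; Enemy_2 is an enemy Blueprint that spins as it advances on a heading taken toward the player's Gun, and sets a score value.
; The construction script scales it up, finds the Gun and stores a look-at movement transform.
; Tick advances that transform along local X and composes a separate yaw spin onto it, in frame-rate-dependent steps without sweep.
; Hits forward to EnemyEventHit; overlapping the Gun changes EnemyState and shakes the camera.
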(event EventTick
  (params (DeltaSeconds :type Float%20%28single-precision%29))
  (|CallParentFunction DeltaSeconds)
  (bind _output_get (Variables|Default|SetRotationZPow (+ (Variables|Default|GetRotationZPow) 5.0)))
  (bind _output_get_2 (Variables|Default|SetMoveTrans (Math|Transform|ComposeTransforms (Math|Transform|MakeTransform "3.000000, 0, 0") (Variables|Default|GetMoveTrans))))
  (Transformation|SetActorTransform (Math|Transform|ComposeTransforms (Math|Transform|MakeTransform "0, 0, 0" (Math|Rotator|MakeRotator 0.0 0.0 _output_get)) _output_get_2) :!pinned true) ; アクタにセット
)

(event Collision|EventHit
  (params (MyComp :type Primitive%20Component%20Object%20Reference) (Other :type Actor%20Object%20Reference) (OtherComp :type Primitive%20Component%20Object%20Reference) (bSelfMoved :type Boolean) (HitLocation :type Vector :default "0, 0, 0") (HitNormal :type Vector :default "0, 0, 0") (NormalImpulse :type Vector :default "0, 0, 0") (Hit :type Hit%20Result%20Structure%20%28by%20ref%29))
  (CallFunction|EnemyEventHit Other HitLocation))

(event Collision|EventActorBeginOverlap
  (params (OtherActor :type Actor%20Object%20Reference))
  (if (== (Utilities|GetClass OtherActor) "/Game/BluePrints/Player/Gun.Gun_C")
    (Variables|Default|SetEnemyState "NewEnumerator1")
    (Class|PlayerController|ClientPlayCameraShake (Game|GetPlayerController 0) "/Game/BluePrints/Generic/CameraShake/PlayerCameraShake.PlayerCameraShake_C" 1.0 "CameraLocal" "0, 0, 0")))

(fn ConstructionScript
  (|CallParentFunction)
  (Transformation|SetActorTransform (Math|Transform|ComposeTransforms (Math|Transform|MakeTransform "0, 0, 0" "0, 0, 0" "3.000000,3.000000,3.000000") (Transformation|GetActorTransform)))
  (bind _outactors (Actor|GetAllActorsOfClass "/Game/BluePrints/Player/Gun.Gun_C")) ; Gun(Player)を検索して\nGunActorへセット
  (Variables|Default|SetgunActor_0 (Utilities|Array|Get(acopy) _outactors))
  (Variables|Default|SetMoveTrans (Math|Transform|MakeTransform (Math|Transform|TransformLocation (Transformation|GetActorTransform) "0, 0, 0") (Math|Interpolation|RInterpTo (Transformation|GetActorRotation) (Math|Rotator|FindLookatRotation (Transformation|GetActorLocation) (Transformation|GetActorLocation (Variables|Default|GetgunActor_0))) (Utilities|Time|GetWorldDeltaSeconds) 1e+02) (Transformation|GetActorScale3D))) ; 移動用の行列セット
  (Variables|Default|SetaddScore 200))